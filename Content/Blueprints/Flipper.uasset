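; Pinball flipper actor that swings between a rest and a raised rotation, set up as a left or right flipper through FlipType.
; The construction script picks mirrored start and end rotations per side and negates the X scale for the right side.
; Flip plays a side-specific sound and eases the Flipper component to its end rotation with MoveComponentTo; Flop returns it over the same FlipTime.
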(event `self.ReceiveBeginPlay`)

(event `Flip`
  (bind _returnvalue (`self.K2_GetActorLocation`))
  (switch `/Game/Blueprints/FlipType` (`self.FlipType`)
    (:`NewEnumerator0`
      (`GameplayStatics.PlaySoundAtLocation` "/Game/Assets/Sounds/Pinball_FlipperLeft_Cue.Pinball_FlipperLeft_Cue" _returnvalue (struct) 1.0 1.0 0.0 null null null))
    (:`NewEnumerator1`
      (`GameplayStatics.PlaySoundAtLocation` "/Game/Assets/Sounds/Pinball_FlipperRight_Cue.Pinball_FlipperRight_Cue" _returnvalue (struct) 1.0 1.0 0.0 null null null)))
  (`KismetSystemLibrary.MoveComponentTo` (`self.Flipper`) (0.0 0.0 0.0) (`self.EndRotation`) false false (`self.Flip Time`)))

(event `Flop`
  (`KismetSystemLibrary.MoveComponentTo` (`self.Flipper`) (0.0 0.0 0.0) (`self.StartRotation`) false false (`self.Flip Time`)))

(fn `UserConstructionScript`
  (set `self.StartRotation` (select `/Game/Blueprints/FlipType` (`self.FlipType`) :`NewEnumerator0` (struct :`Yaw` 20.0) :`NewEnumerator1` (struct :`Yaw` -20.0) :!type "Rotator Structure"))
  (set `self.EndRotation` (select `/Game/Blueprints/FlipType` (`self.FlipType`) :`NewEnumerator0` (struct :`Yaw` -20.0) :`NewEnumerator1` (struct :`Yaw` 20.0) :!type "Rotator Structure"))
  (`SceneComponent.K2_SetRelativeRotation` (`self.Flipper`) (`self.StartRotation`) false false)
  (switch `/Game/Blueprints/FlipType` (`self.FlipType`)
    (:`NewEnumerator1`
      (`SceneComponent.SetRelativeScale3D` (`self.Flipper`) (-1.0 1.0 1.0)))))